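; Player state Blueprint for a two-player chest game of hiding and guessing treasure, driving chest visuals and post-authorization UI.
; It caches every Chest at BeginPlay, then its events show, open and close chests or reveal treasure.
; Chests are found by display name (Chest_1_N, Chest_2_N), with IsPlayerOne selecting the enemy side and pair numbers mapping to two indices.
; Authorization and score events update the AutorizationUI widget.
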(event `self.ReceiveBeginPlay`
  ;[1 1 1] Find all chests on level
  (bind _outactors (`GameplayStatics.GetAllActorsOfClass` "/Game/Blueprints/Chest.Chest_C"))
  (set `self.AllChests` _outactors))

(event `self.ShowOnAutorized`
  ;[1 1 1] Show UI elements after User Autorization
  (`parent.ShowOnAutorized`)
  (bind _asautorization_ui (cast `/Game/Blueprints/AutorizationUI` (`self.userMenu`))
    (:`then`
      (`|ExecutionSequence`
        (:`then_0`
          (`Widget.SetVisibility` (`/Game/Blueprints/AutorizationUI.UserAutorized` _asautorization_ui) "Visible"))
        (:`then_1`
          (`Widget.SetVisibility` (`/Game/Blueprints/AutorizationUI.ScoreInput` _asautorization_ui) "Visible"))
        (:`then_2`
          (`Widget.SetVisibility` (`/Game/Blueprints/AutorizationUI.GetScoreButton` _asautorization_ui) "Visible"))
        (:`then_3`
          (`Widget.SetVisibility` (`/Game/Blueprints/AutorizationUI.SetScoreButton` _asautorization_ui) "Visible"))
        (:`then_4`
          (`Widget.SetVisibility` (`/Game/Blueprints/AutorizationUI.HightScore` _asautorization_ui) "Visible"))
        (:`then_5`
          (`Widget.SetVisibility` (`/Game/Blueprints/AutorizationUI.StartMatchButton` _asautorization_ui) "Visible"))))
    (:`CastFailed`
      (`KismetSystemLibrary.PrintString` "Cast in PlayerState to AutorizeUI failed !!"))))

(event `self.SetPlayerScore`
  (params (newScore :type Integer))
  ;[1 1 1] Temp. Show User Score from GS server
  (`parent.SetPlayerScore` newScore)
  (bind _asautorization_ui (cast `/Game/Blueprints/AutorizationUI` (`self.userMenu`)))
  (`SpinBox.SetValue` (`/Game/Blueprints/AutorizationUI.ScoreInput` _asautorization_ui) (`KismetMathLibrary.Conv_IntToDouble` (`self.GetPlayerScore`))))

(event `self.EnemyChestHideMessage`
  (params (pairNum :type Integer))
  (bind _returnvalue (* pairNum 2))
  (bind _returnvalue_2 (`KismetStringLibrary.Conv_IntToString` _returnvalue))
  (bind _returnvalue_3 (`KismetStringLibrary.Conv_IntToString` (+ _returnvalue 1)))
  ;[1 1 1] When enemy hide treasure , we select right chestst and send Event to them , to animate opening cap
  (`parent.EnemyChestHideMessage` pairNum)
  (`KismetSystemLibrary.PrintString` (`KismetStringLibrary.Concat_StrStr` "Enemy Try to hide chest-pait N " (`KismetStringLibrary.Conv_IntToString` pairNum)) true true (struct :`G` 0.66 :`B` 1.0 :`A` 1.0) 10.0)
  (for _array_element (`self.AllChests`)
    (if (`self.isPlayerOne`)
      (bind _returnvalue_4 (`KismetSystemLibrary.GetDisplayName` _array_element))
      (if (or (`KismetStringLibrary.EqualEqual_StrStr` _returnvalue_4 (`KismetStringLibrary.Concat_StrStr` "Chest_2_" _returnvalue_2)) (`KismetStringLibrary.EqualEqual_StrStr` _returnvalue_4 (`KismetStringLibrary.Concat_StrStr` "Chest_2_" _returnvalue_3)))
        (`/Game/Blueprints/Chest.OpenChest` _array_element false :!label _label))
      (elif (or (`KismetStringLibrary.EqualEqual_StrStr` _returnvalue_4 (`KismetStringLibrary.Concat_StrStr` "Chest_1_" _returnvalue_2)) (`KismetStringLibrary.EqualEqual_StrStr` _returnvalue_4 (`KismetStringLibrary.Concat_StrStr` "Chest_1_" _returnvalue_3)))
        (goto _label)))))

(event `self.OpenChestEvent`
  (params (chestName :type String) (isTreasure :type Boolean))
  ;[1 1 1] Open chest , and show or not treasut in there
  (`parent.OpenChestEvent` chestName false)
  (`KismetSystemLibrary.PrintString` (`KismetStringLibrary.Concat_StrStr` "Player Try to hide in " chestName) true true (struct :`G` 0.66 :`B` 1.0 :`A` 1.0) 10.0)
  (for _array_element (`self.AllChests`)
    (if (`KismetStringLibrary.EqualEqual_StrStr` (`KismetSystemLibrary.GetDisplayName` _array_element) chestName)
      (`/Game/Blueprints/Chest.OpenChest` _array_element isTreasure))))

(event `self.ShowChests`
  ;[1 1 1] Show Chests
  ;;[1 1 1] hide all chest
  (for _array_element (`self.AllChests`)
    (set `/Game/Blueprints/Chest.isChestVisible` false _array_element)
    (`/Game/Blueprints/Chest.SetChestVisibility` _array_element))
  ;;[1 1 1] show conditionals count of chest
  (for _index (range (* (`self.visiblePairs`) 2))
    (for _array_element_2 (`self.AllChests`)
      (bind _returnvalue (`KismetSystemLibrary.GetDisplayName` _array_element_2))
      (if (or (`KismetStringLibrary.EqualEqual_StrStr` _returnvalue (`KismetStringLibrary.Concat_StrStr` "Chest_2_" (`KismetStringLibrary.Conv_IntToString` _index))) (`KismetStringLibrary.EqualEqual_StrStr` _returnvalue (`KismetStringLibrary.Concat_StrStr` "Chest_1_" (`KismetStringLibrary.Conv_IntToString` _index))))
        (set `/Game/Blueprints/Chest.isChestVisible` true _array_element_2)
        (`/Game/Blueprints/Chest.SetChestVisibility` _array_element_2)))))

(event `self.CloseAllChest`
  ;[1 1 1] Close ALL chests
  (for _array_element (`self.AllChests`)
    (`/Game/Blueprints/Chest.CloseChest` _array_element)))

(event `self.ShowTreasureInEnemyChest`
  (params (chestNum :type Integer))
  ;[1 1 1] if player guess Enemy treashure, than we show gold coins in chest
  (for _array_element (`self.AllChests`)
    (if (`self.isPlayerOne`)
      (bind _returnvalue (`KismetSystemLibrary.GetDisplayName` _array_element))
      (if (`KismetStringLibrary.EqualEqual_StrStr` _returnvalue (`KismetStringLibrary.Concat_StrStr` "Chest_2_" (`KismetStringLibrary.Conv_IntToString` chestNum)))
        (`/Game/Blueprints/Chest.SetTreasureVisibility` _array_element true :!label _label_2))
      (elif (`KismetStringLibrary.EqualEqual_StrStr` _returnvalue (`KismetStringLibrary.Concat_StrStr` "Chest_1_" (`KismetStringLibrary.Conv_IntToString` chestNum)))
        (goto _label_2)))))

(fn `UserConstructionScript`)