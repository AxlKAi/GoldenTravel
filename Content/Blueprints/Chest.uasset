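; Clickable chest actor that opens and closes, showing coins inside when it holds treasure.
; Trigger box clicks report the chest's display name to the first player's PlayerState_BP, with a timer-reset DoOnce blocking rapid repeats.
; OpenChest, meant to be called from GameState, and CloseChest are state-guarded and swing the lid through opposing timelines.
; Helpers toggle chest visibility and get player and chest numbers by having PlayerState parse the name.
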(event `self.ReceiveBeginPlay`
  (bind _asplayer_state_bp (cast `/Game/Blueprints/PlayerState_BP` (`Controller.PlayerState` (`GameplayStatics.GetPlayerController` 0)))
    (:`then`
      (`KismetSystemLibrary.PrintString` (`KismetStringLibrary.Concat_StrStr` (`KismetSystemLibrary.GetObjectName` self) " cast to base"))
      (set `self.PlayerStateBaseRef` _asplayer_state_bp))
    (:`CastFailed`
      (`KismetSystemLibrary.PrintString` "Cast from OpenChest to PlayerStateBase failed !" true true (struct :`R` 1.0 :`G` 0.028928 :`A` 1.0) 5.0))))

(event `OpenChest`
  (params (isTreasure :type Boolean :default false))
  (if (not (`self.isChestOpen`))
    (set `self.isChestOpen` true)
    (`self.SetTreasureVisibility` isTreasure)
    (`KismetSystemLibrary.PrintString` "Chest Click")
    (`|ExecutionSequence`
      (:`then_0`
        (bind (_direction _newtrack_1) (`Timeline|CloseChestTimeline` :!via `Stop` :!label _label)
          (:`Update`
            (`self.SetChestCapAngle` _newtrack_1))))
      (:`then_1`
        (bind (_direction_2 _newtrack_0) (`Timeline|Timeline_0` :!via `PlayFromStart` :!label _label_2)
          (:`Update`
            (`self.SetChestCapAngle` _newtrack_0)))))))

(event `CloseChest`
  (if (`self.isChestOpen`)
    (set `self.isChestOpen` false)
    (`self.SetTreasureVisibility` false)
    (`|ExecutionSequence`
      (:`then_0`
        (goto _label_2 :!via `Stop`))
      (:`then_1`
        (goto _label :!via `PlayFromStart`)))))

(event `self.CestTriggerBox.OnClicked`
  (params (TouchedComponent :type "PrimitiveComponent Object Reference") (ButtonPressed :type "Key Structure" :default "AnyKey"))
  (`/Engine/EditorBlueprintResources/StandardMacros.DoOnce` false :!label _label_3
    (:`Completed`
      (`PlayerStateBase.ChestClicked` (`self.PlayerStateBaseRef`) (`KismetSystemLibrary.GetDisplayName` self))
      (`KismetSystemLibrary.K2_SetTimerDelegate` (delegate `FrequentClickProtection`) 0.3))))

(event `FrequentClickProtection`
  (goto _label_3 :!via `Reset`))

(fn `GetPlayerAndChestNumbers`
  (returns (Player :type Integer) (Chest :type Integer))
  (bind _playerstatebaseref (`self.PlayerStateBaseRef`))
  (bind _returnvalue (`KismetSystemLibrary.GetDisplayName` self))
  (bind _returnvalue_2 (`PlayerStateBase.ParseChest` _playerstatebaseref _returnvalue))
  (bind _returnvalue_3 (`PlayerStateBase.ParsePlayer` _playerstatebaseref _returnvalue))
  (return _returnvalue_3 _returnvalue_2))

(fn `SetChestCapAngle`
  (params (Angle :type "Float (double-precision)"))
  (`SceneComponent.K2_SetRelativeRotation` (`self.SM_Prop_Chest_03_Lid`) (`KismetMathLibrary.MakeRotator` Angle) false false))

(fn `SetChestVisibility`
  (bind _ischestvisible (`self.isChestVisible`))
  (`|ExecutionSequence`
    (:`then_0`
      (`SceneComponent.SetVisibility` (`self.SM_Prop_Chest_03`) _ischestvisible false))
    (:`then_1`
      (`SceneComponent.SetVisibility` (`self.SM_Prop_Chest_03_Lid`) _ischestvisible false))
    (:`then_2`
      (`self.SetTreasureVisibility` false))
    (:`then_3`
      (`SceneComponent.SetVisibility` (`self.CestTriggerBox`) _ischestvisible false))))

(fn `SetTreasureVisibility`
  (params (Visible :type Boolean))
  (`|ExecutionSequence`
    (:`then_0`
      (`SceneComponent.SetVisibility` (`self.SM_Item_Coins_02`) Visible false))
    (:`then_1`
      (`SceneComponent.SetVisibility` (`self.SM_Item_Coins_01`) Visible false))))

(fn `UserConstructionScript`)