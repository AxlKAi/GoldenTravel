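; Camera controller Blueprint that plays a demo camera sequence and feeds an FPS readout to the game UI.
; On BeginPlay it caches the player's PlayerState_BP, and on first Tick it grabs the first GameUI widget.
; Each Tick then writes the rounded frame rate into that widget.
; Key 1 or ShowDemo switches the view to the first CineCameraActor found and plays DemoCameraSequence from the start.
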(event `self.ReceiveBeginPlay`
  ;[1 1 1] store reference to PlayerState
  (bind _asplayer_state_bp (cast `/Game/Blueprints/PlayerState_BP` (`Controller.PlayerState` (`GameplayStatics.GetPlayerController` 0)))
    (:`then`
      (`KismetSystemLibrary.PrintString` (`KismetStringLibrary.Concat_StrStr` (`KismetSystemLibrary.GetObjectName` self) " cast to base"))
      (set `self.PlayerStateRef` _asplayer_state_bp))
    (:`CastFailed`
      (`KismetSystemLibrary.PrintString` "Cast from CameraController to PlayerStateBase failed !" true true (struct :`R` 1.0 :`G` 0.028928 :`A` 1.0) 5.0))))

(event `self.ReceiveTick`
  (params (DeltaSeconds :type "Float (single-precision)"))
  (bind _gameuiref (`self.gameUIref`))
  (`|ExecutionSequence`
    (:`then_0`
      ;[1 1 1] Get link to gameUI menu
      (`/Engine/EditorBlueprintResources/StandardMacros.DoOnce` false
        (:`Completed`
          (bind _foundwidgets (`WidgetBlueprintLibrary.GetAllWidgetsOfClass` "/Game/Blueprints/GameUI.GameUI_C" false))
          (set `self.gameUIref` (`KismetArrayLibrary.Array_Get` _foundwidgets)))))
    (:`then_1`
      ;[1 1 1] count and show FPS
      (`/Engine/EditorBlueprintResources/StandardMacros.IsValid` _gameuiref
        (:`Is Valid`
          (set `/Game/Blueprints/GameUI.FPStext` (`KismetTextLibrary.Conv_StringToText` (`KismetStringLibrary.Concat_StrStr` "FPS : " (`KismetTextLibrary.Conv_TextToString` (`KismetTextLibrary.Conv_DoubleToText` (`KismetMathLibrary.Conv_IntToDouble` (`KismetMathLibrary.Round` (/ 1.0 DeltaSeconds))) "HalfToEven")))) _gameuiref))
        (:`Is Not Valid`
          (`KismetSystemLibrary.PrintString` "not vaild GameUIref" true true (struct :`R` 1.0 :`B` 0.015525 :`A` 1.0) 5.0))))))

(event `Key|One`
  (params (Key :type "Key Structure" :default "AnyKey"))
  ;[1 1 1] show camera demo
  (:`Pressed`
    (`KismetSystemLibrary.PrintString` "Start to show demo" :!label _label)
    (bind _returnvalue (`LevelSequencePlayer.CreateLevelSequencePlayer` (`self.DemoCameraSequence`)))
    (`LevelSequencePlayer.SetPlaybackPosition` _returnvalue 0.0)
    (bind _outactors (`GameplayStatics.GetAllActorsOfClass` "/Script/CinematicCamera.CineCameraActor"))
    (`self.SetViewTargetWithBlend` (`KismetArrayLibrary.Array_Get` _outactors))
    (`LevelSequencePlayer.Play` _returnvalue)))

(event `ShowDemo`
  ;[1 1 1] show camera demo
  (goto _label))

(fn `UserConstructionScript`)